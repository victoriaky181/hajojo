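; BP_Tunnel2 is an input-driven tunnel actor with an early rotation setup.
; BeginPlay adds the Controls mapping context to the Enhanced Input local player subsystem.
; RotateLeft prints a debug message, calls SetActorRotation with no rotation wired in, then stores a 120-degree yaw offset in TargetRotation, which nothing here reads.
; RotateRight only prints, and a PlayerController cast is left unconnected.
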(event Input|EnhancedActionEvents|EnhancedInputActionRotateRight
  (params (ActionValue :type Boolean) (ElapsedSeconds :type Float%20%28double-precision%29) (TriggeredSeconds :type Float%20%28double-precision%29) (InputAction :type Input%20Action%20Object%20Reference :default "/Game/Controls/RotateRight.RotateRight"))
  (Development|PrintString "input right"))

(event Input|EnhancedActionEvents|EnhancedInputActionRotateLeft
  (params (ActionValue :type Boolean) (ElapsedSeconds :type Float%20%28double-precision%29) (TriggeredSeconds :type Float%20%28double-precision%29) (InputAction :type Input%20Action%20Object%20Reference :default "/Game/Controls/RotateLeft.RotateLeft"))
  (bind _returnvalue (Transformation|GetActorRotation))
  (Development|PrintString "Rotating Left" true true "(R=0.000000,G=0.660000,B=1.000000,A=1.000000)" 3.0)
  (Transformation|SetActorRotation (Math|Rotator|MakeRotator 0.0 0.0 0.0))
  (Variables|Default|SetTarget%20Rotation (Math|Rotator|MakeRotator (.roll _returnvalue) (.pitch _returnvalue) (+ (.yaw _returnvalue) 1.2e+02))))

(event EventBeginPlay
  (bind _returnvalue (PlayerController|LocalPlayerSubsystems|GetEnhancedInputLocalPlayerSubsystem 0))
  (Utilities|IsValid _returnvalue
    (:Is%20Valid
      (Input|AddMappingContext _returnvalue "/Game/Controls/Controls.Controls" 0 "(bIgnoreAllPressedKeysUntilRelease=True,bForceImmediately=False,bNotifyUserSettings=False)"))))

(event Collision|EventActorBeginOverlap
  (params (OtherActor :type Actor%20Object%20Reference)))

(event EventTick
  (params (DeltaSeconds :type Float%20%28single-precision%29)))

(fn ConstructionScript)