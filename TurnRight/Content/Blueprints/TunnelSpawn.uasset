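; Tunnel segment actor that chains actors at its far attach point as the player moves through, suggesting an endless runner.
; Player overlap on SpawnTrigger spawns an actor at Attachpoint, and overlap on DeleteTrigger destroys this segment.
; ChangeLane drives a timeline that lerps the actor's rotation toward a LanePosition entry, built from an X-axis vector.
; CurretnLaneIndex is read there but never updated in this file.
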(event OnComponentBeginOverlap(DeleteTrigger)
  (params (OverlappedComponent :type Primitive%20Component%20Object%20Reference) (OtherActor :type Actor%20Object%20Reference) (OtherComp :type Primitive%20Component%20Object%20Reference) (OtherBodyIndex :type Integer) (bFromSweep :type Boolean) (SweepResult :type Hit%20Result%20Structure%20%28by%20ref%29))
  (if (== OtherActor (Variables|Default|GetAs%20BP%20Player))
    (Actor|DestroyActor)))

(event OnComponentBeginOverlap(SpawnTrigger)
  (params (OverlappedComponent :type Primitive%20Component%20Object%20Reference) (OtherActor :type Actor%20Object%20Reference) (OtherComp :type Primitive%20Component%20Object%20Reference) (OtherBodyIndex :type Integer) (bFromSweep :type Boolean) (SweepResult :type Hit%20Result%20Structure%20%28by%20ref%29))
  (if (== OtherActor (Variables|Default|GetAs%20BP%20Player))
    (Game|SpawnActorfromClass "TunnelSpawn_C" (Transformation|GetWorldTransform (Variables|Default|GetAttachpoint)) "Undefined" "MultiplyWithRoot" 0 (Game|Player|GetPlayerPawn 0))))

(event Custom|ChangeLane
  (params (ShiftLanes :type Integer))
  (bind _returnvalue (Transformation|GetActorRotation))
  (bind _returnvalue_2 (Math|Rotator|GetRotationXVector _returnvalue))
  (bind (_x _y _z) (Math|Vector|BreakVector _returnvalue_2))
  (Variables|Default|SetTagetLaneIndex (+ ShiftLanes (Variables|Default|GetCurretnLaneIndex)))
  (Variables|Default|SetZYPosition (+ _y _z))
  (bind _changelanes (Timeline|Timeline PlayFromStart)
    (:Update
      (Transformation|SetActorRotation (Math|Conversions|RotationFromXVector (Math|Vector|MakeVector (.X (Math|Vector|BreakVector (Transformation|GetActorLocation))) (Math|Float|Lerp (Variables|Default|GetZYPosition) (Utilities|Array|Get(acopy) (Variables|Default|GetLanePosition) (Variables|Default|GetTagetLaneIndex)) _changelanes) (Math|Float|Lerp (Variables|Default|GetZYPosition) (Utilities|Array|Get(acopy) (Variables|Default|GetLanePosition) (Variables|Default|GetTagetLaneIndex)) _changelanes)))))
    (:Finished
      (Variables|Default|SetTagetLaneIndex (Variables|Default|GetTagetLaneIndex)))))

(event EventBeginPlay
  (bind _asbp_player (Utilities|Casting|CastToBP_Player (Game|Player|GetPlayerPawn 0)))
  (Variables|Default|SetAs%20BP%20Player _asbp_player))

(fn ConstructionScript)

(fn AddFloor
  (return (Transformation|GetWorldTransform (Variables|Default|GetAttachpoint))))

(fn GetAttachPoint
  (return (Transformation|GetWorldTransform (Variables|Default|GetAttachpoint))))