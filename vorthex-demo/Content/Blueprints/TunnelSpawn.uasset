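; TunnelSpawn is a tunnel segment that chains copies of itself and removes itself, apparently for an endless runner.
; SpawnTrigger spawns the next segment at the Arrow transform and DeleteTrigger destroys this one, both only when the overlapping actor matches the AsPlayerStart reference.
; BeginPlay casts that reference from itself, with no other source shown.
; ChangeLane drives a timeline that rotates the segment toward a LanePosition entry, though CurretnLaneIndex is never updated here.
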(event OnComponentBeginOverlap(SpawnTrigger)
  (params (OverlappedComponent :type Primitive%20Component%20Object%20Reference) (OtherActor :type Actor%20Object%20Reference) (OtherComp :type Primitive%20Component%20Object%20Reference) (OtherBodyIndex :type Integer) (bFromSweep :type Boolean) (SweepResult :type Hit%20Result%20Structure%20%28by%20ref%29))
  (if (== OtherActor (Variables|Default|GetAs%20Player%20Start))
    (Game|SpawnActorfromClass "TunnelSpawn_C" (Transformation|GetWorldTransform (Variables|Default|GetArrow)) "Undefined" "MultiplyWithRoot" 0 (Game|GetPlayerCharacter 0))))

(event OnComponentBeginOverlap(DeleteTrigger)
  (params (OverlappedComponent :type Primitive%20Component%20Object%20Reference) (OtherActor :type Actor%20Object%20Reference) (OtherComp :type Primitive%20Component%20Object%20Reference) (OtherBodyIndex :type Integer) (bFromSweep :type Boolean) (SweepResult :type Hit%20Result%20Structure%20%28by%20ref%29))
  (if (== OtherActor (Variables|Default|GetAs%20Player%20Start))
    (Actor|DestroyActor)))

(event Custom|ChangeLane
  (params (ShiftLanes :type Integer))
  (bind _returnvalue (Transformation|GetActorRotation))
  (bind _returnvalue_2 (Math|Rotator|GetRotationXVector _returnvalue))
  (bind (_x _y _z) (Math|Vector|BreakVector _returnvalue_2))
  (Variables|Default|SetTagetLaneIndex (+ ShiftLanes (Variables|Default|GetCurretnLaneIndex)))
  (Variables|Default|SetZYPosition (+ _y _z))
  (bind _changelanes (Timeline|Timeline PlayFromStart)
    (:Update
      (Transformation|SetActorRotation (Math|Conversions|RotationFromXVector (Math|Vector|MakeVector (.X (Math|Vector|BreakVector (Transformation|GetActorLocation))) (Math|Float|Lerp (Variables|Default|GetZYPosition) (Utilities|Array|Get(acopy) (Variables|Default|GetLanePosition) (Variables|Default|GetTagetLaneIndex)) _changelanes) (Math|Float|Lerp (Variables|Default|GetZYPosition) (Utilities|Array|Get(acopy) (Variables|Default|GetLanePosition) (Variables|Default|GetTagetLaneIndex)) _changelanes)))))
    (:Finished
      (Variables|Default|SetTagetLaneIndex (Variables|Default|GetTagetLaneIndex)))))

(event EventBeginPlay
  (bind _asplayer_start (Utilities|Casting|CastToPlayerStart (Variables|Default|GetAs%20Player%20Start)))
  (Variables|Default|SetAs%20Player%20Start _asplayer_start))

(fn ConstructionScript)

(fn Spawnpoint)

(fn GetAttachPoint
  (return (Transformation|GetWorldTransform (Variables|Default|GetArrow))))