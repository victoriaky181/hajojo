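; BP_PlayerShip is a player ship that turns its Cyl component around the roll axis in steps on Rotate input.
; Each input adds TurnRate times the axis value to the current roll, and Rotate_TL eases from that start to the rounded target.
; CanTurn blocks new input until the timeline finishes, so turns never overlap.
; A debug print of the target roll runs on every timeline update.
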(event Input|EnhancedActionEvents|EnhancedInputActionRotate
  (params (ActionValue :type Vector%202D%20Structure) (ElapsedSeconds :type Float%20%28double-precision%29) (TriggeredSeconds :type Float%20%28double-precision%29) (InputAction :type Input%20Action%20Object%20Reference :default "/Game/Controls/Rotate.Rotate"))
  (bind _cyl (Variables|Default|Getcyl))
  (bind _relativerotation (Variables|/Script/Engine.SceneComponent|GetRelativeRotation _cyl))
  (bind (_roll _pitch _yaw) (Math|Rotator|BreakRotator _relativerotation))
  (if (Variables|Default|GetCan%20Turn)
    (Variables|Default|SetCan%20Turn false)
    (Variables|Default|SetCurrent%20Rotation _roll)
    (Variables|Default|SetTarget%20Rotation (+ _roll (* (Variables|Default|GetTurnRate) (.x ActionValue))))
    (bind _alpha (Timeline|Rotate_TL PlayFromStart)
      (:Update
        (Transformation|SetRelativeRotation (Variables|Default|Getcyl) (Math|Rotator|MakeRotator (Math|Float|Lerp (Variables|Default|GetCurrent%20Rotation) (Math|Conversions|ToFloat(Integer) (Math|Float|Round (Variables|Default|GetTarget%20Rotation))) _alpha) _pitch _yaw) false false)
        (Development|PrintString (Utilities|String|ToString(Float) (Variables|Default|GetTarget%20Rotation))))
      (:Finished
        (Variables|Default|SetCurrent%20Rotation (Math|Float|Lerp (Variables|Default|GetCurrent%20Rotation) (Math|Conversions|ToFloat(Integer) (Math|Float|Round (Variables|Default|GetTarget%20Rotation))) _alpha))
        (Variables|Default|SetCan%20Turn true)))))

(event EventBeginPlay)

(event Collision|EventActorBeginOverlap
  (params (OtherActor :type Actor%20Object%20Reference)))

(fn ConstructionScript)